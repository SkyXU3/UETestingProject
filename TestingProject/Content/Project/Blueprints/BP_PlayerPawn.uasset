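; BP_PlayerPawn is a player pawn that moves by setting the physics linear velocity of its ModelMesh every Tick.
; It combines forward/backward and right/left values with the Camera's forward and right vectors, then scales the result by MoveSpeed, so movement depends on camera orientation.
; Only the X and Y of that result feed the new velocity.
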(event EventBeginPlay)

(event Collision|EventActorBeginOverlap
  (params (OtherActor :type Actor%20Object%20Reference)))

(event EventTick
  (params (DeltaSeconds :type Float%20%28single-precision%29))
  (bind _returnvalue (Input|AxisValues|GetForward/Backward))
  (bind _returnvalue_2 (Input|AxisValues|GetRight/Left))
  (bind _camera (Variables|Default|GetCamera))
  (bind _modelmesh (Variables|Default|GetModelMesh))
  (bind _movespeed (Variables|Default|GetMoveSpeed))
  (bind _returnvalue_3 (Math|Vector|GetForwardVector _camera))
  (bind _returnvalue_4 (Math|Vector|GetRightVector _camera))
  (bind _returnvalue_5 (+ _returnvalue_4 _returnvalue_2))
  (bind _returnvalue_6 (+ _returnvalue _returnvalue_3))
  (bind _returnvalue_7 (* _returnvalue_6 _returnvalue_5))
  (bind _returnvalue_8 (* _returnvalue_7 _movespeed))
  (Physics|GetPhysicsLinearVelocity _modelmesh "None")
  (Physics|SetPhysicsLinearVelocity _modelmesh (Math|Vector|MakeVector (.x _returnvalue_8) (.y _returnvalue_8) 0.0) false "None"))

(fn ConstructionScript)
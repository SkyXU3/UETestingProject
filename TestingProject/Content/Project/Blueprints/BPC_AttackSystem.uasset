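; BPC_AttackSystem is a player attack component that runs a melee combo from the IA_Attack input.
; BaseAttack buffers input through SaveCombo and, when not attacking, dispatches on AttackIndex to Attack1, which plays a delayed, DoOnce-gated montage and advances the index.
; SytheAttackCombo either consumes the buffered input to re-dispatch or resets the combo, though only the first attack is wired.
; Each permitted press also applies test damage to BP_Player.
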(event Custom|BaseAttack
  ;[0 0 0] Attack
  (if (Variables|Default|GetisAttacking)
    (Variables|Default|SetsaveCombo true)
    (else
      (Variables|Default|SetsaveCombo true)
      (switch int (Variables|Default|GetAttackIndex)
        (:0
          (CallFunction|Attack1))))))

(event Custom|SytheAttackCombo
  ;[0 0 0] ComboExtend
  (if (Variables|Default|GetsaveCombo)
    (Variables|Default|SetsaveCombo false)
    (switch int (Variables|Default|GetAttackIndex)
      (:0
        (CallFunction|Attack1)))
    (else
      (CallFunction|StopCombo))))

(event Custom|StopCombo
  ;[0 0 0] StopCombo
  (Variables|Default|SetisAttacking false)
  (Variables|Default|SetAttackIndex 0))

(event Custom|Attack1
  ;[0 0 0] Attack1
  (Utilities|FlowControl|DoOnce false :!label _label
    (:Completed
      (Utilities|FlowControl|Delay 0.2)
      (Animation|Montage|PlayMontage (Variables|Default|GetPlayerMesh) 0
        (:then
          (Variables|Default|SetAttackIndex 1)
          (goto _label Reset))))))

(event Input|EnhancedActionEvents|EnhancedInputActionIA_Attack
  (params (ActionValue :type Boolean) (ElapsedSeconds :type Float%20%28double-precision%29) (TriggeredSeconds :type Float%20%28double-precision%29) (InputAction :type Input%20Action%20Object%20Reference :default "/Game/Project/Input/IA_Attack.IA_Attack"))
  ;[0 0 0] Input
  (:Started
    (if (Variables|Default|GetcanAttack)
      (CallFunction|BaseAttack)
      ;[0 0 0] TestDmg
      (bind _returnvalue (Actor|GetActorOfClass "/Game/Project/Blueprints/BP_Player.BP_Player_C"))
      (Game|Damage|ApplyDamage _returnvalue 1e+01 0 0))))

(event EventBeginPlay
  (bind _asbp_player (Utilities|Casting|CastToBP_Player (Components|GetOwner)))
  (Variables|Default|SetPlayerMeshTest _asbp_player))